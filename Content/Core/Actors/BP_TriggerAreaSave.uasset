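; BP_TriggerAreaSave is a checkpoint actor that records where the main character respawns.
; When a MainCharacter overlaps its Box, it writes the RespawnPoint's world location to LastLocation on the GI_GMTK game instance.
; It then disables the Box's collision, making it one-shot, and plays the checkpoint activation animation on its skeletal mesh.
; A material "Light Intensity" change is present but never runs.
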(event `self.Box.OnComponentBeginOverlap`
  (params (OverlappedComponent :type "PrimitiveComponent Object Reference") (OtherActor :type "Actor Object Reference") (OtherComp :type "PrimitiveComponent Object Reference") (OtherBodyIndex :type Integer) (bFromSweep :type Boolean) (SweepResult :type "HitResult Structure (by ref)"))
  (if (`GameplayStatics.ObjectIsA` OtherActor "/Script/GMTK_Jam_2025.MainCharacter")
    (bind _asgi_gmtk (cast `/Game/Core/GameInstance/GI_GMTK` (`GameplayStatics.GetGameInstance`)))
    (set `/Game/Core/GameInstance/GI_GMTK.LastLocation` (`SceneComponent.K2_GetComponentLocation` (`self.RespawnPoint`)) _asgi_gmtk)
    (`PrimitiveComponent.SetCollisionEnabled` (`self.Box`) "NoCollision")
    (`SkeletalMeshComponent.PlayAnimation` (`self.SkeletalMesh`) "/Game/Art/SKELETAL/Checkpoint/CheckPoint_Activation_Anim.CheckPoint_Activation_Anim" false)))

(fn `UserConstructionScript`)