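; BP_MainCharacter is a character Blueprint that fakes a drop shadow under the player while airborne.
; On BeginPlay a looping 0.03-second timer fires CastShadow.
; CastShadow shows ShadowDecal only while the movement component reports falling, then traces downward from the capsule on the Visibility channel and moves the decal to the impact location.
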(event `self.ReceiveBeginPlay`
  ;[1 1 1] Move decal to create a fake shadow effect
  ;;[0.1192 0.09891 0.5365] Fire event looping with timer
  (`KismetSystemLibrary.K2_SetTimerDelegate` (delegate `CastShadow`) 0.03 true))

(event `CastShadow`
  (bind _returnvalue (`SceneComponent.K2_GetComponentLocation` (`self.CapsuleComponent`)))
  ;[1 1 1] Move decal to create a fake shadow effect
  (`SceneComponent.SetVisibility` (`self.ShadowDecal`) (`NavMovementComponent.IsFalling` (`self.CharacterMovement`)) false)
  (bind _outhit (`KismetSystemLibrary.LineTraceSingle` :`Start` _returnvalue :`End` (- _returnvalue (`KismetMathLibrary.MakeVector` 0.0 0.0 2000.0)) :`TraceChannel` "TraceTypeQuery1" :`DrawTime` 0.5))
  ;;[0.1192 0.09891 0.5365] Move the decal to the linetrace impact location
  (`SceneComponent.K2_SetWorldLocation` (`self.ShadowDecal`) (`.Location` (`GameplayStatics.BreakHitResult` _outhit)) false false))

(fn `UserConstructionScript`)