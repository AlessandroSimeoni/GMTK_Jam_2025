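; Gameplay ability that runs the player character's wall run.
; On activation it zeroes vertical velocity, applies wall gravity and speed from the character's AttributeSet, and plays a right or left montage based on IsRightWall.
; A per-tick ability task then calls DoWallRun with the character.
; Ending the ability restores default gravity and walk speed from the same AttributeSet.
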(event `self.K2_ActivateAbility`
  (bind _returnvalue (`GameplayStatics.GetPlayerCharacter` 0))
  (bind _asbp_main_character (cast `/Game/Core/Character/BP_MainCharacter` _returnvalue :!pure true))
  (bind _charactermovement (`Character.CharacterMovement` _returnvalue))
  (bind (_velocity_x _velocity_y) (`KismetMathLibrary.BreakVector` (`MovementComponent.Velocity` _charactermovement)))
  (`KismetSystemLibrary.PrintString` "START WALL RUN")
  (bind _output_get (set `self.As BP Main Character` _asbp_main_character))
  (set `MovementComponent.Velocity` (`KismetMathLibrary.MakeVector` _velocity_x _velocity_y) _charactermovement)
  (bind _attributeset (`MainCharacter.AttributeSet` _output_get))
  (bind _wallgravityscale_basevalue (break `GameplayAttributeData` (`PlayerAttributeSet.WallGravityScale` _attributeset)))
  (set `CharacterMovementComponent.GravityScale` _wallgravityscale_basevalue _charactermovement)
  (bind _wallplayerspeed_basevalue (break `GameplayAttributeData` (`PlayerAttributeSet.WallPlayerSpeed` _attributeset)))
  (set `CharacterMovementComponent.MaxWalkSpeed` _wallplayerspeed_basevalue _charactermovement)
  (`AbilityTask_PlayMontageAndWait.CreatePlayMontageAndWaitProxy` "None" (select `bool` (`MainCharacter.IsRightWall` _asbp_main_character) :`false` "/Game/Core/Character/Animations/AM_Rokko_WallRun_SX.AM_Rokko_WallRun_SX" :`true` "/Game/Core/Character/Animations/AM_Rokko_WallRun_DX.AM_Rokko_WallRun_DX" :!type "AnimMontage Object Reference")
    (:`then`
      (`CharacterAbilityTask_OnTick.AbilityTaskOnTick`
        (:`OnTick`
          (`self.DoWallRun` (`self.As BP Main Character`)))))))

(event `self.K2_OnEndAbility`
  (params (bWasCancelled :type Boolean))
  (bind _charactermovement (`Character.CharacterMovement` (`GameplayStatics.GetPlayerCharacter` 0)))
  (bind _attributeset (`MainCharacter.AttributeSet` (stale `self.K2_ActivateAbility` _output_get)))
  (bind _defaultgravityscale_basevalue (break `GameplayAttributeData` (`PlayerAttributeSet.DefaultGravityScale` _attributeset)))
  (set `CharacterMovementComponent.GravityScale` _defaultgravityscale_basevalue _charactermovement)
  (bind _playerspeed_basevalue (break `GameplayAttributeData` (`PlayerAttributeSet.PlayerSpeed` _attributeset)))
  (set `CharacterMovementComponent.MaxWalkSpeed` _playerspeed_basevalue _charactermovement)
  (`KismetSystemLibrary.PrintString` "FINE WALL RUN"))