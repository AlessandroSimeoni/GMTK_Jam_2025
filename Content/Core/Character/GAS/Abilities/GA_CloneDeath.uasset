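; Gameplay ability that handles the player's clone death and returns the character to the last checkpoint.
; On activation it disables movement and controls, plays the death montage, and spawns a shell through MainCharacter when the montage completes before ending the ability.
; On end it safe-teleports the player to the location saved in GI_GMTK, raised by capsule half-height, then restores walking and controls.
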(event `self.K2_ActivateAbility`
  (`KismetSystemLibrary.PrintString` "CLONE DEATH")
  (`CharacterMovementComponent.SetMovementMode` (`Character.CharacterMovement` (`GameplayStatics.GetPlayerCharacter` 0)) "MOVE_None" 0)
  (`CharacterController.ToggleControls` (cast `CharacterController` (`GameplayStatics.GetPlayerController` 0) :!pure true) false)
  ;[1 1 1] Clone death montage
  (`AbilityTask_PlayMontageAndWait.CreatePlayMontageAndWaitProxy` "None" "/Game/Core/Character/Animations/AM_Death.AM_Death"
    (:`OnCompleted`
      (`MainCharacter.SpawnShell` (cast `MainCharacter` (`GameplayStatics.GetPlayerCharacter` 0) :!pure true))
      (`self.K2_EndAbility`))))

(event `self.K2_OnEndAbility`
  (params (bWasCancelled :type Boolean))
  (bind _returnvalue (`GameplayStatics.GetPlayerCharacter` 0))
  ;[1 1 1] Teleport player to last checkpoint and toggle controls
  (bind _asgi_gmtk (cast `/Game/Core/GameInstance/GI_GMTK` (`GameplayStatics.GetGameInstance`)))
  (`MainCharacter.SafeTeleport` (cast `MainCharacter` _returnvalue :!pure true) (+ (`/Game/Core/GameInstance/GI_GMTK.LastLocation` _asgi_gmtk) (* (`CapsuleComponent.CapsuleHalfHeight` (`Character.CapsuleComponent` _returnvalue)) (`KismetMathLibrary.Vector_Up`))))
  (`CharacterMovementComponent.SetMovementMode` (`Character.CharacterMovement` _returnvalue) "MOVE_Walking" 0)
  (`CharacterController.ToggleControls` (cast `CharacterController` (`GameplayStatics.GetPlayerController` 0) :!pure true) true))