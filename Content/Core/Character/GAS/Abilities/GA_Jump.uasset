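; GA_Jump is a Gameplay Ability that makes the player's BP_MainCharacter jump.
; On activation it clears the character's LastMovementDirection, calls Jump and ends immediately.
; A disconnected tick-task branch, which never runs, would check CanWallRun while falling, activate GA_WallRun on success, and end upon wall run or landing.
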(event `self.K2_ActivateAbility`
  (bind _output_get (set `self.As BP Main Character` (cast `/Game/Core/Character/BP_MainCharacter` (`GameplayStatics.GetPlayerCharacter` 0) :!pure true)))
  (set `MainCharacter.LastMovementDirection` (0.0 0.0 0.0) _output_get)
  (`Character.Jump` _output_get)
  (`self.K2_EndAbility`))