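; GA_Test is a test Gameplay Ability that runs per-tick logic until the player character is no longer falling.
; On activation it casts player character 0 to BP_MainCharacter and starts an AbilityTaskOnTick task that prints a debug string each tick.
; Once the movement component reports not falling, it ends the task and the ability, then prints a completion message.
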(event `self.K2_ActivateAbility`
  (set `self.As BP Main Character` (cast `/Game/Core/Character/BP_MainCharacter` (`GameplayStatics.GetPlayerCharacter` 0) :!pure true))
  (bind _asynctaskproxy (`CharacterAbilityTask_OnTick.AbilityTaskOnTick`)
    (:`OnTick`
      (`KismetSystemLibrary.PrintString` "Hello" true true (struct :`G` 0.66 :`B` 1.0 :`A` 1.0) 0.25)
      (if (not (`NavMovementComponent.IsFalling` (`Character.CharacterMovement` (`self.As BP Main Character`))))
        (`GameplayTask.EndTask` _asynctaskproxy)
        (`self.K2_EndAbility`)
        (`KismetSystemLibrary.PrintString` "FINITOOPOOOOO" true true (struct :`G` 0.66 :`B` 1.0 :`A` 1.0) 0.25)))))