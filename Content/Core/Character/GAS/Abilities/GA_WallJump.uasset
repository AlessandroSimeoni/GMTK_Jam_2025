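; Gameplay ability that launches the player character off a wall for a wall jump.
; It rotates the character's forward vector by the attribute set's yaw, signed by wall side, then by its pitch.
; The result, scaled by the wall jump power attribute, overrides velocity via LaunchCharacter, and the ability ends after a brief delay.
; It also prints a debug string, while a debug line draw sits unreachable.
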(event `self.K2_ActivateAbility`
  (bind _returnvalue (`GameplayStatics.GetPlayerCharacter` 0))
  (bind _asbp_main_character (cast `/Game/Core/Character/BP_MainCharacter` _returnvalue :!pure true))
  (bind _attributeset (`MainCharacter.AttributeSet` _asbp_main_character))
  (bind _walljumpyaw_basevalue (break `GameplayAttributeData` (`PlayerAttributeSet.WallJumpYaw` _attributeset)))
  (bind _walljumppitch_basevalue (break `GameplayAttributeData` (`PlayerAttributeSet.WallJumpPitch` _attributeset)))
  (bind _walljumppower_basevalue (break `GameplayAttributeData` (`PlayerAttributeSet.WallJumpPower` _attributeset)))
  (`KismetSystemLibrary.PrintString` "WALL JUMPO")
  (bind _output_get (set `self.PlayerForward` (`Actor.GetActorForwardVector` _returnvalue)))
  (bind _returnvalue_2 (`KismetMathLibrary.RotateAngleAxis` _output_get (* (select `bool` (`MainCharacter.IsRightWall` _asbp_main_character) :`false` 1.0 :`true` -1.0) _walljumpyaw_basevalue) (`Actor.GetActorUpVector` _returnvalue)))
  (bind _output_get_2 (set `self.PlayerForward` (`KismetMathLibrary.RotateAngleAxis` _returnvalue_2 (* _walljumppitch_basevalue -1.0) (`KismetMathLibrary.Cross_VectorVector` (`KismetMathLibrary.Vector_Up`) _returnvalue_2))))
  (`Character.LaunchCharacter` _returnvalue (* _output_get_2 _walljumppower_basevalue) true true)
  (`KismetSystemLibrary.Delay` 0.1)
  (`self.K2_EndAbility`))