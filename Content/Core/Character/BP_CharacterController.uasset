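; Player controller that toggles the game's pause state and pause menu through a PauseGame event.
; Pausing creates and stores a W_Pause widget, shows the mouse cursor and switches to Game and UI input focused on the resume button.
; Unpausing removes that widget and its WCommands sub-widget, restoring game-only input only when WCommands is valid; the cursor is not hidden again here.
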(event `self.PauseGame`
  (bind _pausewidget (`self.PauseWidget`))
  (if (`GameplayStatics.IsGamePaused`)
    (`GameplayStatics.SetGamePaused` false)
    (`/Engine/EditorBlueprintResources/StandardMacros.IsValid` _pausewidget
      (:`Is Valid`
        (`Widget.RemoveFromParent` _pausewidget)
        (bind _w_commands (`/Game/Core/UI/Pause/W_Pause.W_Commands` (`self.PauseWidget`))
          (:`then`
            (`Widget.RemoveFromParent` _w_commands)
            (`WidgetBlueprintLibrary.SetInputMode_GameOnly` self))
          (:`else`))))
    (else
      (`GameplayStatics.SetGamePaused` true)
      (bind _returnvalue (`|CreateWidget` "/Game/Core/UI/Pause/W_Pause.W_Pause_C" self))
      (`UserWidget.AddToViewport` _returnvalue 0)
      (set `self.PauseWidget` _returnvalue)
      (`WidgetBlueprintLibrary.SetInputMode_GameAndUIEx` self (`/Game/Core/UI/Pause/W_Pause.ResumeButton` _returnvalue))
      (set `self.bShowMouseCursor` true))))

(fn `UserConstructionScript`)