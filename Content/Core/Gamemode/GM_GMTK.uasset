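; Game mode for a timed level that runs from the level start to the victory screen and time save.
; BeginPlay stores the player's foot position in the game instance, adds the HUD, plays an optional soundtrack and binds to the level's win trigger.
; On win, it pauses, matches the score to a data-asset threshold phrase for the victory widget, then saves the current time under the level name.
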(event `self.ReceiveBeginPlay`
  (bind _returnvalue (`GameplayStatics.GetPlayerCharacter` 0))
  (set `/Game/Core/GameInstance/GI_GMTK.LastLocation` (+ (`self.K2_GetActorLocation` _returnvalue) (* (`CapsuleComponent.CapsuleHalfHeight` (`Character.CapsuleComponent` _returnvalue)) (`KismetMathLibrary.Vector_Down`))) (cast `/Game/Core/GameInstance/GI_GMTK` (`GameplayStatics.GetGameInstance`) :!pure true))
  (bind _returnvalue_2 (`|CreateWidget` "/Game/Core/UI/HUD/W_HUD.W_HUD_C" (`GameplayStatics.GetPlayerController` 0)))
  (`UserWidget.AddToViewport` _returnvalue_2 0)
  (bind _returnvalue_3 (`GameplayStatics.GetActorOfClass` "/Game/Core/Actors/BP_WinTrigger.BP_WinTrigger_C"))
  (bind _output_get (set `self.WinTrigger` _returnvalue_3))
  (add `/Game/Core/Actors/BP_WinTrigger.Win` _output_get (delegate `Win_Event`))
  (bind _soundtrack (`self.Soundtrack`)
    (:`then`
      (`GameplayStatics.PlaySound2D` _soundtrack 1.0 1.0 0.0 null null false))
    (:`else`)))

(event `self.ReceiveTick`
  (params (DeltaSeconds :type "Float (single-precision)")))

(event `Win_Event`
  (bind _returnvalue (`GameplayStatics.GetPlayerController` 0))
  (bind _returnvalue_2 (subsystem `SaveSystem`))
  (bind _currenttime (`self.CurrentTime`))
  (`GameplayStatics.SetGamePaused` true)
  (bind _returnvalue_3 (`|CreateWidget` "/Game/Core/UI/Win/W_Victory.W_Victory_C" _returnvalue))
  (set `self.WinWidget` _returnvalue_3)
  (`WidgetBlueprintLibrary.SetInputMode_UIOnlyEx` _returnvalue _returnvalue_3)
  (set `PlayerController.bShowMouseCursor` true (`GameplayStatics.GetPlayerController` 0))
  (bind _returnvalue_4 (`self.ReturnScore`))
  (for _array_element (`ThresholdDataAsset.Thresholds` (`self.ThresholdDataAsset`))
    (if (== (break `TimeThresoldStruct` _array_element) _returnvalue_4)
      (`/Game/Core/UI/Win/W_Victory.SetTime` (`self.WinWidget`) _currenttime)
      (`/Game/Core/UI/Win/W_Victory.SetPhrase` (`self.WinWidget`) (`.ThresholdPhrase` (break `TimeThresoldStruct` _array_element)))
      (break)))
  (`UserWidget.AddToViewport` (`self.WinWidget`) 0)
  (bind _returnvalue_5 (`SaveSystem.LoadGame` _returnvalue_2))
  (bind _returnvalue_6 (`GameplayStatics.GetCurrentLevelName` true))
  (`GMTKSave.SaveTimeToLevel` _returnvalue_5 _returnvalue_6 _currenttime)
  (`SaveSystem.SaveGame` _returnvalue_2))

(fn `UserConstructionScript`)