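; Test actionable actor that shuttles between its BeginPlay location and LocationB while activated, then returns to its start.
; ActivateActor starts two chained timelines at a Speed play rate, each lerping from the current location rather than a fixed origin.
; Their Update pins run a StoppingTime delay, then check StillOverlapping to continue the loop or stop it.
; DeactivateActor only clears that flag; StopLoopingMovement then plays a third timeline back to the start.
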(event `self.ReceiveBeginPlay`
  (set `self.LocationA` (`self.K2_GetActorLocation`)))

(event `self.ActivateActor`
  ;[1 1 1] Activation
  (set `self.StillOverlapping` true)
  (`self.LoopingMovement`))

(event `self.DeactivateActor`
  ;[1 1 1] Activation
  (set `self.StillOverlapping` false))

(event `LoopingMovement`
  (bind _speed (`self.Speed`))
  (bind _stoppingtime (`self.StoppingTime`))
  ;[1 1 1] Looping
  (bind (_direction _distance) (`Timeline|Timeline` :!via `PlayFromStart` :!label _label)
    (:`Update`
      (`TimelineComponent.SetPlayRate` (`self.Timeline`) _speed)
      (`self.K2_SetActorLocation` (`KismetMathLibrary.VLerp` (`self.K2_GetActorLocation`) (`self.LocationB`) _distance))
      (`KismetSystemLibrary.Delay` _stoppingtime)
      (if (`self.StillOverlapping`)
        (bind (_direction_2 _distance_2) (`Timeline|Timeline_0` :!via `PlayFromStart`)
          (:`Update`
            (`TimelineComponent.SetPlayRate` (`self.Timeline_0`) _speed)
            (`self.K2_SetActorLocation` (`KismetMathLibrary.VLerp` (`self.K2_GetActorLocation`) (`self.LocationA`) _distance_2))
            (`KismetSystemLibrary.Delay` _stoppingtime)
            (if (`self.StillOverlapping`)
              (goto _label :!via `PlayFromStart`)
              (else
                (`self.StopLoopingMovement`)))))
        (else
          (`self.StopLoopingMovement`))))))

(event `StopLoopingMovement`
  ;[1 1 1] StopLooping
  (`TimelineComponent.Stop` (`self.Timeline_0`))
  (`TimelineComponent.Stop` (`self.Timeline`))
  (if (`self.StillOverlapping`)
    (`self.LoopingMovement`)
    (else
      (bind (_direction _distance) (`Timeline|Timeline_1` :!via `PlayFromStart`)
        (:`Update`
          (`TimelineComponent.SetPlayRate` (`self.Timeline_1`) (`self.Speed`))
          (`self.K2_SetActorLocation` (`KismetMathLibrary.VLerp` (`self.K2_GetActorLocation`) (`self.LocationA`) _distance)))))))

(fn `UserConstructionScript`
  (`parent.UserConstructionScript`))