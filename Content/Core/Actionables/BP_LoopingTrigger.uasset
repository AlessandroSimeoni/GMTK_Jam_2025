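; BP_LoopingTrigger is an actor that moves back and forth between its starting location and LocationB in an endless loop.
; BeginPlay stores the start as LocationA and plays two timelines that chain into each other, each setting its play rate from Speed.
; Each update lerps from the current location toward its target by the Distance track, then runs a StoppingTime delay that leads to the opposite timeline.
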(event `self.ReceiveBeginPlay`
  (set `self.LocationA` (`self.K2_GetActorLocation`))
  (`self.LoopingMovement`))

(event `LoopingMovement`
  (bind _speed (`self.Speed`))
  (bind _stoppingtime (`self.StoppingTime`))
  ;[1 1 1] Looping
  (bind (_direction _distance) (`Timeline|Timeline_0` :!via `PlayFromStart` :!label _label)
    (:`Update`
      (`TimelineComponent.SetPlayRate` (`self.Timeline_0`) _speed)
      (`self.K2_SetActorLocation` (`KismetMathLibrary.VLerp` (`self.K2_GetActorLocation`) (`self.LocationB`) _distance))
      (`KismetSystemLibrary.Delay` _stoppingtime)
      (bind (_direction_2 _distance_2) (`Timeline|Timeline_1` :!via `PlayFromStart`)
        (:`Update`
          (`TimelineComponent.SetPlayRate` (`self.Timeline_1`) _speed)
          (`self.K2_SetActorLocation` (`KismetMathLibrary.VLerp` (`self.K2_GetActorLocation`) (`self.LocationA`) _distance_2))
          (`KismetSystemLibrary.Delay` _stoppingtime)
          (goto _label :!via `PlayFromStart`))))))

(fn `UserConstructionScript`)