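; BP_TestActiveSpikesMoving is an activatable actor, named as a test moving spike hazard, that slides between its starting location and LocationB.
; ActivateActor and DeactivateActor set a direction flag that PlatformMoving reads and flips.
; A Timeline drives a location lerp without sweep, with its play rate set from Speed.
; Forward movement starts after a WaitingTime delay, while deactivation reverses immediately.
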(event `self.ReceiveBeginPlay`
  (set `self.LocationA` (`self.K2_GetActorLocation`)))

(event `self.ActivateActor`
  (`self.MoveToPositionB`))

(event `MoveToPositionB`
  ;[1 1 1] Moving Bool A-B
  (set `self.MovetoB` true)
  (`self.PlatformMoving`))

(event `MoveToPositionA`
  ;[1 1 1] Moving Bool B-A
  (set `self.MovetoB` false)
  (`self.PlatformMoving`))

(event `self.DeactivateActor`
  (`self.MoveToPositionA`))

(event `PlatformMoving`
  ;[1 1 1] Moving Platform
  (if (`self.MovetoB`)
    (set `self.MovetoB` false)
    (`KismetSystemLibrary.Delay` (`self.WaitingTime`))
    (bind (_direction _distance) (`Timeline|Timeline` :!label _label)
      (:`Update`
        (`TimelineComponent.SetPlayRate` (`self.Timeline`) (`self.Speed`))
        (`self.K2_SetActorLocation` (`KismetMathLibrary.VLerp` (`self.LocationA`) (`self.LocationB`) _distance))))
    (else
      (set `self.MovetoB` true)
      (goto _label :!via `Reverse`))))

(fn `UserConstructionScript`
  (`parent.UserConstructionScript`))