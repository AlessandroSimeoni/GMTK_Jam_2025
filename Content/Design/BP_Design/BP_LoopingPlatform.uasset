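; BP_LoopingPlatform is a platform that shuttles between its starting location and LocationB while StillOverlapping is true.
; On BeginPlay it stores its start and binds LoopingMovement to each detector's Looping event.
; Timelines lerp the location out and back, with Speed serving as both play rate and delay.
; When overlap ends, StopLoopingMovement lerps from LocationB to the start if displaced, but sets Timeline0's rate rather than its own timeline's.
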(event `self.ReceiveBeginPlay`
  ;[1 1 1] Looping
  (set `self.LocationA` (`self.K2_GetActorLocation`))
  (for _ (`self.Detectors`)
    (add `self.Looping` (delegate `LoopingMovement`))))

(event `LoopingMovement`
  (bind _speed (`self.Speed`))
  (bind _stilloverlapping (`self.StillOverlapping`))
  ;[1 1 1] Looping
  (if _stilloverlapping
    (bind (_direction _distance) (`Timeline|Timeline_2` :!via `PlayFromStart` :!label _label)
      (:`Update`
        (`TimelineComponent.SetPlayRate` (`self.Timeline_2`) _speed)
        (`self.K2_SetActorLocation` (`KismetMathLibrary.VLerp` (`self.LocationA`) (`self.LocationB`) _distance))
        (if _stilloverlapping
          (`KismetSystemLibrary.Delay` _speed)
          (bind (_direction_2 _distance_2) (`Timeline|Timeline_0` :!via `PlayFromStart`)
            (:`Update`
              (`TimelineComponent.SetPlayRate` (`self.Timeline_0`) _speed)
              (`self.K2_SetActorLocation` (`KismetMathLibrary.VLerp` (`self.LocationB`) (`self.LocationA`) _distance_2))
              (`KismetSystemLibrary.Delay` _speed)
              (if _stilloverlapping
                (goto _label :!via `PlayFromStart`)
                (else
                  (`self.StopLoopingMovement`)))))
          (else
            (`self.StopLoopingMovement`)))))
    (else
      (`self.StopLoopingMovement`))))

(event `StopLoopingMovement`
  ;[1 1 1] StopLooping
  (bind _output_get (set `self.IsInPlace` (`KismetMathLibrary.EqualExactly_VectorVector` (`self.K2_GetActorLocation`) (`self.LocationA`))))
  (if (not _output_get)
    (bind (_direction _distance) (`Timeline|Timeline`)
      (:`Update`
        (`TimelineComponent.SetPlayRate` (`self.Timeline_0`) (`self.Speed`))
        (`self.K2_SetActorLocation` (`KismetMathLibrary.VLerp` (`self.LocationB`) (`self.LocationA`) _distance))))))

(fn `UserConstructionScript`)