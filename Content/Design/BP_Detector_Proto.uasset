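; Prototype detector actor that activates linked platforms when an actor overlaps it.
; Begin overlap sets StillOverlapping and calls the overlap function on each normal platform in PlatformsNormali; end overlap clears the flag and calls their end-overlap function.
; Looping platforms receive LoopB then LoopA calls, gated by that flag, from a loop nested inside the normal-platform loop, so they are triggered once per normal platform.
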(event `self.ReceiveActorBeginOverlap`
  (params (OtherActor :type "Actor Object Reference"))
  (bind _stilloverlapping (`self.StillOverlapping`))
  ;[1 1 1] Normal Platform Activation
  (for _array_element (`self.PlatformsNormali`)
    (set `self.StillOverlapping` true)
    (`/Game/Design/BP_MovingPlatform.OverlapDetector` _array_element)
    ;[1 1 1] Loop Activation
    (for _array_element_2 (`self.LoopingPlatforms`)
      (if _stilloverlapping
        (`/Game/Design/BP_LoopingPlatform.LoopB` _array_element_2)
        (if _stilloverlapping
          (`/Game/Design/BP_LoopingPlatform.LoopA` _array_element_2))))))

(event `self.ReceiveActorEndOverlap`
  (params (OtherActor :type "Actor Object Reference"))
  ;[1 1 1] Normal Platform Activation
  (for _array_element (`self.PlatformsNormali`)
    (set `self.StillOverlapping` false)
    (`/Game/Design/BP_MovingPlatform.EndOverlapDetector` _array_element)))

(fn `UserConstructionScript`)