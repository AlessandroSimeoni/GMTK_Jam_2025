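; Moving platform actor that travels between its starting location and LocationB once its Looping dispatcher fires.
; BeginPlay stores the start position as LocationA and binds Looping1 to that dispatcher.
; Looping1 plays a timeline that lerps the actor's location at a play rate set by Speed.
; Delays of WaitingTime chained from timeline updates trigger a second timeline in reverse, which in turn reverses the first.
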(event `self.ReceiveBeginPlay`
  (set `self.LocationA` (`self.K2_GetActorLocation`))
  ;[1 1 1] Looping
  (add `self.Looping` (delegate `Looping1`)))

(event `Looping1`
  (bind _waitingtime (`self.WaitingTime`))
  (bind _speed (`self.Speed`))
  ;[1 1 1] Looping
  (bind (_direction _distance) (`Timeline|Timeline_2` :!label _label)
    (:`Update`
      (`TimelineComponent.SetPlayRate` (`self.Timeline_2`) _speed)
      (`self.K2_SetActorLocation` (`KismetMathLibrary.VLerp` (`self.LocationA`) (`self.LocationB`) _distance))
      (`KismetSystemLibrary.Delay` _waitingtime)
      (bind (_direction_2 _distance_2) (`Timeline|Timeline_0` :!via `Reverse`)
        (:`Update`
          (`TimelineComponent.SetPlayRate` (`self.Timeline_0`) _speed)
          (`self.K2_SetActorLocation` (`KismetMathLibrary.VLerp` (`self.LocationA`) (`self.LocationB`) _distance_2))
          (`KismetSystemLibrary.Delay` _waitingtime)
          (goto _label :!via `Reverse`))))))

(fn `UserConstructionScript`)